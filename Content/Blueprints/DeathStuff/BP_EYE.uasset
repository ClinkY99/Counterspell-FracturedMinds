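; BP_EYE is an actor that shows an animated 2D eyes flipbook when looked at.
; Tick turns SpawnPoint toward the player character with a 90-degree yaw offset, billboarding anything attached to it.
; LookedAt spawns a PaperFlipbookActor attached to that point and assigns the Eyes flipbook.
; NotLookedAt destroys every PaperFlipbookActor in the level, not just the one it spawned.
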(event `self.ReceiveTick`
  (params (DeltaSeconds :type "Float (single-precision)"))
  (bind _asb_horrer_jam_character (cast `bHorrerJamCharacter` (`GameplayStatics.GetPlayerCharacter` 0)))
  (`SceneComponent.K2_SetWorldRotation` (`self.SpawnPoint`) (`KismetMathLibrary.MakeRotator` (.roll (`KismetMathLibrary.FindLookAtRotation` (`self.K2_GetActorLocation`) (`self.K2_GetActorLocation` _asb_horrer_jam_character))) (.pitch (`KismetMathLibrary.FindLookAtRotation` (`self.K2_GetActorLocation`) (`self.K2_GetActorLocation` _asb_horrer_jam_character))) (+ (.yaw (`KismetMathLibrary.FindLookAtRotation` (`self.K2_GetActorLocation`) (`self.K2_GetActorLocation` _asb_horrer_jam_character))) 90.0)) false false))

(event `LookedAt`
  (bind _returnvalue (`|SpawnActorFromClass` "/Script/Paper2D.PaperFlipbookActor" (`SceneComponent.K2_GetComponentToWorld` (`self.SpawnPoint`)) "Undefined" "MultiplyWithRoot" null null))
  (`self.K2_AttachToComponent` _returnvalue (`self.SpawnPoint`) "None" "SnapToTarget" "SnapToTarget" "SnapToTarget" true)
  (set `self.Flibook` _returnvalue)
  (`PaperFlipbookComponent.SetFlipbook` (`PaperFlipbookActor.RenderComponent` _returnvalue) "/Game/Blueprints/DeathStuff/EyeTextures/Eyes.Eyes"))

(event `NotLookedAt`
  (bind _outactors (`GameplayStatics.GetAllActorsOfClass` "/Script/Paper2D.PaperFlipbookActor"))
  (for _array_element _outactors
    (`self.K2_DestroyActor` _array_element)))

(fn `UserConstructionScript`)