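; BP_EndSceneEyes is an actor that spawns an eyes flipbook, apparently for the end scene, and keeps itself turned toward the player.
; Tick rotates the root to look at the player character, adding a yaw offset to align it.
; SpawnEyes waits a random few seconds, then spawns a separate non-looping PaperFlipbookActor at this actor's current transform, so staggering multiple instances' appearances.
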(event `self.ReceiveTick`
  (params (DeltaSeconds :type "Float (single-precision)"))
  (bind _asb_horrer_jam_character (cast `bHorrerJamCharacter` (`GameplayStatics.GetPlayerCharacter` 0)))
  (`SceneComponent.K2_SetWorldRotation` (`self.DefaultSceneRoot`) (`KismetMathLibrary.MakeRotator` (.roll (`KismetMathLibrary.FindLookAtRotation` (`self.K2_GetActorLocation`) (`self.K2_GetActorLocation` _asb_horrer_jam_character))) (.pitch (`KismetMathLibrary.FindLookAtRotation` (`self.K2_GetActorLocation`) (`self.K2_GetActorLocation` _asb_horrer_jam_character))) (+ (.yaw (`KismetMathLibrary.FindLookAtRotation` (`self.K2_GetActorLocation`) (`self.K2_GetActorLocation` _asb_horrer_jam_character))) 90.0)) false false))

(event `SpawnEyes`
  (`KismetSystemLibrary.Delay` (`KismetMathLibrary.RandomFloatInRange` 0.0 7.0))
  (bind _returnvalue (`|SpawnActorFromClass` "/Script/Paper2D.PaperFlipbookActor" (`self.GetTransform`) "Undefined" "MultiplyWithRoot" null null))
  (bind _rendercomponent (`PaperFlipbookActor.RenderComponent` _returnvalue))
  (`PaperFlipbookComponent.SetLooping` _rendercomponent false)
  (`PaperFlipbookComponent.SetFlipbook` _rendercomponent "/Game/Blueprints/DeathStuff/EyeTextures/Eyes.Eyes"))

(fn `UserConstructionScript`)