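; Trigger-box actor that spawns an eye, then takes over the first-person camera to face it on a later overlap.
; The first box overlap spawns BP_EYE at the LookAtMe point and sets a flag.
; Subsequent overlaps switch input to UI-only, disable the camera's pawn control rotation, and run the LookAtEye timeline to lerp it from the character's rotation toward LookAtMe.
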(event `self.Box.OnComponentBeginOverlap`
  (params (OverlappedComponent :type "PrimitiveComponent Object Reference") (OtherActor :type "Actor Object Reference") (OtherComp :type "PrimitiveComponent Object Reference") (OtherBodyIndex :type Integer) (bFromSweep :type Boolean) (SweepResult :type "HitResult Structure (by ref)"))
  (bind _returnvalue_location (`KismetMathLibrary.BreakTransform` (`SceneComponent.K2_GetComponentToWorld` (`self.LookAtMe`))))
  (bind _asbp_first_person_character (cast `/Game/FirstPerson/Blueprints/BP_FirstPersonCharacter` (`GameplayStatics.GetPlayerCharacter` 0) :!pure true))
  (bind _firstpersoncameracomponent (`bHorrerJamCharacter.FirstPersonCameraComponent` _asbp_first_person_character))
  (if (`self.second time?`)
    (`WidgetBlueprintLibrary.SetInputMode_UIOnlyEx` (`GameplayStatics.GetPlayerController` 0) null "DoNotLock" true)
    (set `self.StartRot` (`self.K2_GetActorRotation` _asbp_first_person_character))
    (set `CameraComponent.bUsePawnControlRotation` false _firstpersoncameracomponent)
    (bind (_direction _camera) (`Timeline|LookAtEye`)
      (:`Update`
        (`SceneComponent.K2_SetWorldRotation` _firstpersoncameracomponent (`KismetMathLibrary.RLerp` (`self.StartRot`) (`KismetMathLibrary.FindLookAtRotation` (`self.K2_GetActorLocation` _asbp_first_person_character) (.location (`SceneComponent.K2_GetComponentToWorld` (`self.LookAtMe`)))) _camera) false false)))
    (else
      (set `self.second time?` true)
      (`|SpawnActorFromClass` "/Game/Blueprints/DeathStuff/BP_EYE.BP_EYE_C" (`KismetMathLibrary.MakeTransform` _returnvalue_location) "Undefined" "MultiplyWithRoot" null null))))

(fn `UserConstructionScript`)