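; BP_EndCutscene is a trigger actor that runs the ending cutscene when the first-person player overlaps its box.
; On overlap it starts the credits song, switches to UI-only input and detaches the camera from control rotation.
; A timeline lerps the camera from the player's starting rotation toward a LOOKIELOOKIE target.
; When it finishes, every BP_EndSceneEyes spawns its eyes, and the UBP_GoodEnding widget appears after a delay.
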(event `self.Box.OnComponentBeginOverlap`
  (params (OverlappedComponent :type "PrimitiveComponent Object Reference") (OtherActor :type "Actor Object Reference") (OtherComp :type "PrimitiveComponent Object Reference") (OtherBodyIndex :type Integer) (bFromSweep :type Boolean) (SweepResult :type "HitResult Structure (by ref)"))
  (bind _asbp_first_person_character (cast `/Game/FirstPerson/Blueprints/BP_FirstPersonCharacter` (`GameplayStatics.GetPlayerCharacter` 0) :!pure true))
  (bind _firstpersoncameracomponent (`bHorrerJamCharacter.FirstPersonCameraComponent` _asbp_first_person_character))
  (bind _asbp_first_person_character_2 (cast `/Game/FirstPerson/Blueprints/BP_FirstPersonCharacter` OtherActor))
  (bind _returnvalue (`GameplayStatics.SpawnSound2D` "/Game/Music/OST_5_Credit_Song.OST_5_Credit_Song" 1.0 1.0 0.0 null))
  (set `self.CreditsSong` _returnvalue)
  (`WidgetBlueprintLibrary.SetInputMode_UIOnlyEx` (`GameplayStatics.GetPlayerController` 0) null "DoNotLock" true)
  (set `CameraComponent.bUsePawnControlRotation` false (`bHorrerJamCharacter.FirstPersonCameraComponent` _asbp_first_person_character_2))
  (set `self.StartRot` (`self.K2_GetActorRotation` _asbp_first_person_character))
  (set `CameraComponent.bUsePawnControlRotation` false _firstpersoncameracomponent)
  (bind (_direction _camera) (`Timeline|Timeline`)
    (:`Update`
      (`SceneComponent.K2_SetWorldRotation` _firstpersoncameracomponent (`KismetMathLibrary.RLerp` (`self.StartRot`) (`KismetMathLibrary.FindLookAtRotation` (`self.K2_GetActorLocation` _asbp_first_person_character) (.location (`SceneComponent.K2_GetComponentToWorld` (`self.LOOKIELOOKIE`)))) _camera) false false))
    (:`Finished`
      (bind _outactors (`GameplayStatics.GetAllActorsOfClass` "/Game/Blueprints/DeathStuff/BP_EndSceneEyes.BP_EndSceneEyes_C"))
      (for _array_element _outactors
        (`/Game/Blueprints/DeathStuff/BP_EndSceneEyes.SpawnEyes` (cast `/Game/Blueprints/DeathStuff/BP_EndSceneEyes` _array_element :!pure true)))
      (`KismetSystemLibrary.Delay` 10.0)
      (bind _returnvalue_2 (`|CreateWidget` "/Game/Blueprints/UI/UBP_GoodEnding.UBP_GoodEnding_C"))
      (`UserWidget.AddToViewport` _returnvalue_2 0))))

(fn `UserConstructionScript`)