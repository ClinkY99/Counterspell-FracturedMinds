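; BP_TapePlayer is an actor that plays a given tape's audio at its own location.
; PlayTape checks that the tape has a valid sound, stores it as the current tape, flags playback and spawns the sound.
; When the audio finishes, a bound event plays an AfterTape sound for all but one special tape ID, then clears the playing state and current tape.
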(event `self.playTape`
  (params (tapeToPlay :type "TapeDataStruct Structure"))
  (bind (_tapesoundassets _tapeid) (break `TapeDataStruct` tapeToPlay))
  (`/Engine/EditorBlueprintResources/StandardMacros.IsValid` _tapesoundassets
    (:`Is Valid`
      (set `self.tapeBeingPlayed` tapeToPlay)
      (set `self.bIsPlaying` true)
      (bind _returnvalue (`GameplayStatics.SpawnSoundAtLocation` _tapesoundassets (`self.K2_GetActorLocation`) (struct) 0.5 1.0 0.0 null null))
      (add `AudioComponent.OnAudioFinished` _returnvalue (delegate `OnAudioFinished_Event`)))))

(event `OnAudioFinished_Event`
  (if (!= (`.tapeID` (break `TapeDataStruct` (stale `self.playTape` tapeToPlay))) 5)
    (`GameplayStatics.SpawnSoundAtLocation` "/Game/SFX/Interactables/SoundCues/AfterTape.AfterTape" (`self.K2_GetActorLocation`) (struct) 1.0 1.0 0.0 null null))
  (set `self.bIsPlaying` false)
  (set `self.tapeBeingPlayed` (struct)))

(fn `UserConstructionScript`)