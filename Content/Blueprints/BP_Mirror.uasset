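; BP_Mirror is an interactable actor that stages a scare or reveal moment, forcing the first-person player to look at a spawned eye.
; Interacting switches input to UI-only and spawns BP_EYE at the EYESPAWN point.
; It detaches the camera from pawn control rotation, then the LOOKATEYE timeline blends it from the character's rotation toward that point.
; Nothing here restores input or camera control afterwards.
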(event `self.Interacted`
  (bind _asbp_first_person_character (cast `/Game/FirstPerson/Blueprints/BP_FirstPersonCharacter` (`GameplayStatics.GetPlayerCharacter` 0) :!pure true))
  (bind _location (.location (`SceneComponent.K2_GetComponentToWorld` (`self.EYESPAWN`))))
  (bind _firstpersoncameracomponent (`bHorrerJamCharacter.FirstPersonCameraComponent` _asbp_first_person_character))
  (`WidgetBlueprintLibrary.SetInputMode_UIOnlyEx` (`GameplayStatics.GetPlayerController` 0) null "DoNotLock" true)
  (`|SpawnActorFromClass` "/Game/Blueprints/DeathStuff/BP_EYE.BP_EYE_C" (`KismetMathLibrary.MakeTransform` _location) "Undefined" "MultiplyWithRoot" null null)
  (set `self.StartRot` (`self.K2_GetActorRotation` _asbp_first_person_character))
  (set `CameraComponent.bUsePawnControlRotation` false _firstpersoncameracomponent)
  (bind (_direction _newtrack_0) (`Timeline|LOOKATEYE`)
    (:`Update`
      (`SceneComponent.K2_SetWorldRotation` _firstpersoncameracomponent (`KismetMathLibrary.RLerp` (`self.StartRot`) (`KismetMathLibrary.FindLookAtRotation` (`self.K2_GetActorLocation` _asbp_first_person_character) _location) _newtrack_0) false false))))

(fn `UserConstructionScript`)