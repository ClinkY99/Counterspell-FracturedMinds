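; Door actor Blueprint that swings open and closed around a RotationPoint component, with sound.
; It stores the starting rotation on BeginPlay, and a timeline lerps from it to a 90-degree yaw offset.
; OpenDoor plays the timeline and CloseDoor reverses it, each updating IsOpen and playing a non-spatial 2D sound.
; A PlaySound event plays the locked-door sound by ID, though the lock logic itself is not here.
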(event `self.ReceiveBeginPlay`
  (set `self.StartingRot` (`SceneComponent.K2_GetComponentRotation` (`self.rotationPoint`))))

(event `self.openDoor`
  (bind (_startingrot_roll _startingrot_pitch _startingrot_yaw) (`KismetMathLibrary.BreakRotator` (`self.StartingRot`)))
  (set `self.bIsOpen` true)
  (`GameplayStatics.PlaySound2D` "/Game/SFX/Interactables/SoundWaves/Door_open.Door_open" 1.0 1.0 0.0 null null)
  (bind (_direction _rotation) (`Timeline|Open/CloseDoor` :!label _label)
    (:`Update`
      (`SceneComponent.K2_SetWorldRotation` (`self.rotationPoint`) (`KismetMathLibrary.RLerp` (`self.StartingRot`) (`KismetMathLibrary.MakeRotator` _startingrot_roll _startingrot_pitch (+ _startingrot_yaw 90.0)) _rotation) false false))))

(event `self.closeDoor`
  (set `self.bIsOpen` false)
  (`GameplayStatics.PlaySound2D` "/Game/SFX/Interactables/SoundWaves/Door_close.Door_close" 1.0 1.0 0.0 null null)
  (goto _label :!via `Reverse`))

(event `self.playSound`
  (params (ID :type Integer))
  (switch `int` ID
    (:`0`
      (`GameplayStatics.PlaySound2D` "/Game/SFX/Interactables/SoundCues/LockedDoor.LockedDoor" 1.0 1.0 0.0 null null))))

(fn `UserConstructionScript`)